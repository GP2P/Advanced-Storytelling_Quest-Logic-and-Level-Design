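; Glass sliding door for Level1 that opens when the first-person character overlaps it and closes when the character leaves.
; Begin and end overlap events cast to BP_FirstPersonCharacter, then use MoveComponentTo to slide the Cube component sideways along its relative Y axis or back to the origin.
; An InProximity flag guards both events so the door only moves on a change of state.
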(event Collision|EventActorBeginOverlap
  (params (OtherActor :type Actor%20Object%20Reference))
  (if (not (Variables|Default|GetIn%20Proximity))
    (Utilities|Casting|CastToBP_FirstPersonCharacter OtherActor)
    (Variables|Default|SetIn%20Proximity true)
    (Components|MoveComponentTo (Variables|Default|GetCube) "0,200.000000, 0" "0, 0, 0" false false 0.2 false)))

(event Collision|EventActorEndOverlap
  (params (OtherActor :type Actor%20Object%20Reference))
  (if (Variables|Default|GetIn%20Proximity)
    (Utilities|Casting|CastToBP_FirstPersonCharacter OtherActor)
    (Variables|Default|SetIn%20Proximity false)
    (Components|MoveComponentTo (Variables|Default|GetCube) "0, 0, 0" "0, 0, 0" false false 0.2 false)))

(fn ConstructionScript)