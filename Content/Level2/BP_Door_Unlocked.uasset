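; A Level 2 door that opens in two stages as the first-person player character enters its trigger box.
; The first overlap plays one skeletal mesh animation and sets a second-stage flag.
; The next overlap plays a second animation and marks the door open, so later overlaps do nothing.
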(event OnComponentBeginOverlap(Box)
  (params (OverlappedComponent :type Primitive%20Component%20Object%20Reference) (OtherActor :type Actor%20Object%20Reference) (OtherComp :type Primitive%20Component%20Object%20Reference) (OtherBodyIndex :type Integer) (bFromSweep :type Boolean) (SweepResult :type Hit%20Result%20Structure%20%28by%20ref%29))
  (Utilities|Casting|CastToBP_FirstPersonCharacter_Level2 OtherActor)
  (if (not (Variables|Default|GetIsOpen))
    (if (Variables|Default|GetInSecondStage)
      (Components|Animation|PlayAnimation (Variables|SkeletalMeshActor|GetSkeletalMeshComponent) "/Game/Horror_pack/Animation/Door/Door_stm_160-199_.Door_stm_160-199_" false)
      (Variables|Default|SetIsOpen true)
      (else
        (Components|Animation|PlayAnimation (Variables|SkeletalMeshActor|GetSkeletalMeshComponent) "/Game/Horror_pack/Animation/Door/Door_stm_143-160_.Door_stm_143-160_" false)
        (Variables|Default|SetInSecondStage true)))))

(fn ConstructionScript)